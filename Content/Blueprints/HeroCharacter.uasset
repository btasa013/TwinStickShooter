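; Player hero for a twin-stick shooter that moves on world axes, aims, fires and handles its own death.
; On BeginPlay it spawns a weapon on the mesh's GunSocket and records its transform as the game mode's spawn point.
; Look input past a dead zone sets control rotation and pulls the trigger.
; Death costs a life, then after a delay destroys hero and weapon and either respawns or saves the score and opens GameOver.
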(event `self.ReceiveBeginPlay`
  (bind _mesh (`self.Mesh`))
  (`|ExecutionSequence`
    (:`then_0`
      ;[1 1 1] Spawn Weapon
      (bind _returnvalue (`|SpawnActorFromClass` "/Game/Blueprints/Weapon.Weapon_C" (`SceneComponent.K2_GetComponentToWorld` _mesh) "Undefined" "OverrideRootScale" null null))
      (bind _output_get (set `self.Weapon` _returnvalue))
      (`self.K2_AttachToComponent` _output_get _mesh "GunSocket" "SnapToTarget" "SnapToTarget" "KeepWorld" true))
    (:`then_1`
      ;[1 1 1] Set Spawn Transform
      (bind _astwin_stick_mode (cast `/Game/Blueprints/GameModes/TwinStickMode` (`GameplayStatics.GetGameMode`)))
      (bind _output_get_2 (set `self.GameMode` _astwin_stick_mode))
      (set `/Game/Blueprints/GameModes/TwinStickMode.PlayerSpawnTransform` (`self.GetTransform`) _output_get_2))))

(event `InputAxis|MoveUp`
  (params (AxisValue :type "Float (single-precision)"))
  ;[1 1 1] Player Movement
  (`self.AddMovementInput` (1.0 0.0 0.0) AxisValue))

(event `InputAxis|LookUp`
  (params (AxisValue :type "Float (single-precision)"))
  (bind _weapon (`self.Weapon`))
  ;[1 1 1] Player Turn
  (bind _returnvalue (`KismetMathLibrary.MakeVector` AxisValue (stale `InputAxis|LookRight` AxisValue)))
  (if (> (`KismetMathLibrary.VSize` _returnvalue) 0.25) :!label _label
    (`Controller.SetControlRotation` (`self.GetController`) (`KismetMathLibrary.Conv_VectorToRotator` _returnvalue))
    (`/Game/Blueprints/Weapon.PullTrigger` _weapon)
    (else
      (`/Game/Blueprints/Weapon.ReleaseTrigger` _weapon))))

(event `InputAxis|LookRight`
  (params (AxisValue :type "Float (single-precision)"))
  ;[1 1 1] Player Turn
  (goto _label))

(event `InputAxis|MoveRight`
  (params (AxisValue :type "Float (single-precision)"))
  ;[1 1 1] Player Movement
  (`self.AddMovementInput` (0.0 1.0 0.0) AxisValue))

(event `/Game/Blueprints/iDamageable.AffectHealth`
  (params (Delta :type "Float (single-precision)"))
  ;[1 1 1] Affect Health
  (if (not (`self.IsDead`))
    (`self.CalculateHealth` Delta)
    (if (`self.IsDead`)
      (`self.DisableInput` null)
      (bind _result (`/Engine/EditorBlueprintResources/StandardMacros.DecrementInt` (`/Game/Blueprints/GameModes/TwinStickMode.Lifes` (`self.GameMode`)))
        (:`  `
          (`KismetSystemLibrary.Delay` 3.0)
          (`self.K2_DestroyActor` self)
          (`self.K2_DestroyActor` (`self.Weapon`))
          (if (<= _result 0)
            (bind _astwin_stick_shooter_instance (cast `/Game/Blueprints/TwinStickShooterInstance` (`GameplayStatics.GetGameInstance`)))
            (set `/Game/Blueprints/TwinStickShooterInstance.FinalScore` (`/Game/Blueprints/GameModes/TwinStickMode.Score` (`self.GameMode`)) _astwin_stick_shooter_instance)
            (`GameplayStatics.OpenLevel` "GameOver")
            (else
              (`/Game/Blueprints/GameModes/TwinStickMode.RespawnPlayer` (`self.GameMode`)))))))))

(fn `UserConstructionScript`
  (`parent.UserConstructionScript`))