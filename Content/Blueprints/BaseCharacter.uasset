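; BaseCharacter is a character base Blueprint that tracks health and death state.
; The construction script sets Health to MaxHealth.
; CalculateHealth adds a signed Delta to Health without clamping, then calls CalculateDead, which sets IsDead when Health is zero or below.
; The event graph has no active logic, and nothing in this file calls CalculateHealth or reacts to death.
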(fn `CalculateDead`
  (set `self.IsDead` (<= (`self.Health`) 0.0)))

(fn `CalculateHealth`
  (params (Delta :type "Float (double-precision)"))
  (set `self.Health` (+ Delta (`self.Health`)))
  (`self.CalculateDead`))

(fn `UserConstructionScript`
  (set `self.Health` (`self.MaxHealth`)))