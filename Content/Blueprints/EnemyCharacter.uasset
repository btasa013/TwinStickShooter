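; Enemy character for a twin-stick shooter that shoots on a timer and deals repeated contact damage to the hero.
; On BeginPlay it spawns a weapon with enemy projectiles, attaches it to the gun socket and fires on a looping timer.
; Overlapping the hero starts a damage timer.
; Death awards score, disables some collision, detaches the controller and destroys enemy and weapon after a delay; construction tints the body.
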(event `self.ReceiveBeginPlay`
  (bind _mesh (`self.Mesh`))
  ;[1 1 1] Spawn Weapon
  (bind _returnvalue (`|SpawnActorFromClass` "/Game/Blueprints/Weapon.Weapon_C" (`SceneComponent.K2_GetComponentToWorld` _mesh) "Undefined" "OverrideRootScale" null null))
  (set `/Game/Blueprints/Weapon.Projectile` "/Game/Blueprints/EnemyProjectile.EnemyProjectile_C" _returnvalue)
  (bind _output_get (set `self.Weapon` _returnvalue))
  (`self.K2_AttachToComponent` _output_get _mesh "GunSocket" "SnapToTarget" "SnapToTarget" "KeepWorld" true)
  (`KismetSystemLibrary.K2_SetTimer` null "FireWeapon" 3.0 true))

(event `FireWeapon`
  ;[1 1 1] Fire Weapon
  (`/Game/Blueprints/Weapon.Fire` (`self.Weapon`)))

(event `/Game/Blueprints/iDamageable.AffectHealth`
  (params (Delta :type "Float (single-precision)"))
  (bind _capsulecomponent (`self.CapsuleComponent`))
  ;[1 1 1] Affect Health
  (`self.CalculateHealth` Delta)
  (if (`self.IsDead`)
    (bind _astwin_stick_mode (cast `/Game/Blueprints/GameModes/TwinStickMode` (`GameplayStatics.GetGameMode`)))
    (`/Game/Blueprints/GameModes/TwinStickMode.IncrementScore` _astwin_stick_mode (`self.Score`))
    (`PrimitiveComponent.SetCollisionResponseToChannel` _capsulecomponent "ECC_WorldDynamic" "ECR_Ignore")
    (`PrimitiveComponent.SetCollisionResponseToChannel` _capsulecomponent "ECC_Pawn" "ECR_Ignore")
    (`self.DetachFromControllerPendingDestroy`)
    (`KismetSystemLibrary.K2_ClearTimer` null "FireWeapon")
    (`KismetSystemLibrary.Delay` 3.0)
    (`self.K2_DestroyActor` self)
    (`self.K2_DestroyActor` (`self.Weapon`))))

(event `self.ReceiveActorBeginOverlap`
  (params (OtherActor :type "Actor Object Reference"))
  ;[1 1 1] Collision Start
  (bind _ashero_character (cast `/Game/Blueprints/HeroCharacter` OtherActor))
  (set `self.Hero` _ashero_character)
  (`KismetSystemLibrary.K2_SetTimer` null "DamageTheHero" (/ 1.0 (`self.AttacksPerSecond`)) true))

(event `DamageTheHero`
  ;[1 1 1] Damage The Hero
  (`/Game/Blueprints/HeroCharacter.AffectHealth` (`self.Hero`) (`self.Damage`)))

(event `self.ReceiveActorEndOverlap`
  (params (OtherActor :type "Actor Object Reference"))
  ;[1 1 1] Collision End
  (if (== OtherActor (`self.Hero`))
    (`KismetSystemLibrary.K2_ClearTimer` null "DamageTheHero")))

(fn `UserConstructionScript`
  (`parent.UserConstructionScript`)
  (bind _returnvalue (`PrimitiveComponent.CreateDynamicMaterialInstance` (`self.Mesh`) 0 null "None"))
  (bind _output_get (set `self.DynamicMaterial` _returnvalue))
  (`MaterialInstanceDynamic.SetVectorParameterValue` _output_get "BodyColor" (`self.EnemyColor`)))